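; BP_Key is a coloured key pickup that the first-person character collects by touching it.
; The construction script gives the mesh a blue, yellow or red material from KeyColour.
; On box overlap, it overwrites the character's Key map with a single KeyColour-to-KeyPickedup entry, replacing any existing entries, then destroys itself.
; A HasKey assignment is left unconnected and never runs.
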(event `self.Box.OnComponentBeginOverlap`
  (params (OverlappedComponent :type "PrimitiveComponent Object Reference") (OtherActor :type "Actor Object Reference") (OtherComp :type "PrimitiveComponent Object Reference") (OtherBodyIndex :type Integer) (bFromSweep :type Boolean) (SweepResult :type "HitResult Structure (by ref)"))
  (bind _asbp_first_person_character (cast `/Game/FirstPerson/Blueprints/BP_FirstPersonCharacter` OtherActor))
  (`|VariableSetRef` (`/Game/FirstPerson/Blueprints/BP_FirstPersonCharacter.Key` _asbp_first_person_character) (`|MakeMap` (`self.KeyColour`) (`self.KeyPickedup`)))
  (`self.K2_DestroyActor`))

(fn `UserConstructionScript`
  (switch `/Game/Blueprints/e_KeyTypes` (`self.KeyColour`)
    (:`NewEnumerator0`
      (`PrimitiveComponent.SetMaterial` (`self.StaticMesh`) 0 "/Game/Materials/M_Blue.M_Blue"))
    (:`NewEnumerator1`
      (`PrimitiveComponent.SetMaterial` (`self.StaticMesh`) 0 "/Game/Materials/M_Yellow.M_Yellow"))
    (:`NewEnumerator2`
      (`PrimitiveComponent.SetMaterial` (`self.StaticMesh`) 0 "/Game/Materials/M_Red.M_Red"))))