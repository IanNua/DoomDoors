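; Parent door Blueprint with three behaviours chosen by DoorType: locked, interactable or key-gated.
; The construction script sets the door's label text and material, colour-coding key doors by KeyType (blue, yellow, red).
; When the player overlaps the box, locked doors print a refusal and interactable doors destroy themselves.
; Key doors look up their KeyType in the character's Key map, then either destroy themselves or print a prompt.
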(event `self.Box.OnComponentBeginOverlap`
  (params (OverlappedComponent :type "PrimitiveComponent Object Reference") (OtherActor :type "Actor Object Reference") (OtherComp :type "PrimitiveComponent Object Reference") (OtherBodyIndex :type Integer) (bFromSweep :type Boolean) (SweepResult :type "HitResult Structure (by ref)"))
  (bind _asbp_first_person_character (cast `/Game/FirstPerson/Blueprints/BP_FirstPersonCharacter` OtherActor :!pure true))
  (bind _keytype (`self.KeyType`))
  (if (== OtherActor (`GameplayStatics.GetPlayerCharacter` 0))
    (switch `/Game/Blueprints/E_TypesofDoors` (`self.DoorType`)
      (:`NewEnumerator0`
        (`KismetSystemLibrary.PrintString` "This door doesn't open HA!"))
      (:`NewEnumerator1`
        (`self.K2_DestroyActor` self))
      (:`NewEnumerator2`
        (switch `/Game/Blueprints/e_KeyTypes` _keytype
          (:`NewEnumerator0`
            (`self.FindDoorKey` _keytype _asbp_first_person_character))
          (:`NewEnumerator1`
            (`self.FindDoorKey` _keytype _asbp_first_person_character))
          (:`NewEnumerator2`
            (`self.FindDoorKey` _keytype _asbp_first_person_character)))))))

(fn `FindDoorKey`
  (params (Key :type "/Game/Blueprints/e_KeyTypes Enum (by ref)") (self2 :type "/Game/FirstPerson/Blueprints/BP_FirstPersonCharacter Object Reference"))
  (if (`BlueprintMapLibrary.Map_Find` (`/Game/FirstPerson/Blueprints/BP_FirstPersonCharacter.Key` self2) Key)
    (`self.K2_DestroyActor` self)
    (else
      (`KismetSystemLibrary.PrintString` "GET THE KEY!"))))

(fn `Set Door Text`
  (params (Value :type "Text (by ref)"))
  (`TextRenderComponent.K2_SetText` (`self.TextRender`) Value))

(fn `UserConstructionScript`
  (switch `/Game/Blueprints/E_TypesofDoors` (`self.DoorType`)
    (:`NewEnumerator0`
      (`self.Set Door Text` (`self.Text1`))
      (`PrimitiveComponent.SetMaterial` (`self.StaticMesh`) 0 "/Game/LevelPrototyping/Materials/M_FlatCol.M_FlatCol" :!label _label))
    (:`NewEnumerator1`
      (`self.Set Door Text` (`self.Text2`))
      (goto _label))
    (:`NewEnumerator2`
      (`self.Set Door Text` (`self.Text3`))
      (switch `/Game/Blueprints/e_KeyTypes` (`self.KeyType`)
        (:`NewEnumerator0`
          (`PrimitiveComponent.SetMaterial` (`self.StaticMesh`) 0 "/Game/Materials/M_Blue.M_Blue"))
        (:`NewEnumerator1`
          (`PrimitiveComponent.SetMaterial` (`self.StaticMesh`) 0 "/Game/Materials/M_Yellow.M_Yellow"))
        (:`NewEnumerator2`
          (`PrimitiveComponent.SetMaterial` (`self.StaticMesh`) 0 "/Game/Materials/M_Red.M_Red"))))))